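; Cell is an actor that occupies a grid cell on the game field of a Snake game.
; On BeginPlay it caches the SnakeGameMode, which supplies the field size and cell-to-world conversion.
; MoveToCell clamps the requested coordinates to the field bounds, stores them as CurrentCell and sets the actor's location to that cell's position without sweeping.
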(event EventBeginPlay
  (bind _assnake_game_mode (Utilities|Casting|CastToSnakeGameMode (Game|GetGameMode)))
  (Variables|Default|SetSnakeGameMode _assnake_game_mode))

(event Collision|EventActorBeginOverlap
  (params (OtherActor :type Actor%20Object%20Reference)))

(event EventTick
  (params (DeltaSeconds :type Float%20%28single-precision%29)))

(fn ConstructionScript)

(fn MovetoCell
  (params (Cell :type Vector%202D%20Structure))
  (bind (_x _y) (Math|Vector2D|BreakVector2D Cell))
  (bind _snakegamemode (Variables|Default|GetSnakeGameMode))
  (bind _gamefieldsize (Variables|/Game/Blueprints/SnakeGameMode.SnakeGameMode_C|GetGameFieldSize _snakegamemode))
  (bind _returnvalue (- _gamefieldsize "(X=1.000000,Y=1.000000)"))
  (bind (_x_2 _y_2) (Math|Vector2D|BreakVector2D _returnvalue))
  (bind _output_get (Variables|Default|SetCurrentCell (Math|Vector2D|MakeVector2D (Math|Float|Clamp(Float) _x 0.0 _x_2) (Math|Float|Clamp(Float) _y 0.0 _y_2))))
  (bind _position (Default|CelltoPosition (Variables|Default|GetSnakeGameMode) _output_get))
  (Transformation|SetActorLocation _position false false))