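; Player-controlled snake actor that moves cell by cell across the grid defined by SnakeGameMode.
; WASD sets the move direction, and Tick advances one cell whenever the MoveFrequency interval has elapsed in real time.
; MoveToCell clamps the target cell to the game field, then converts it to a world position through the game mode.
; CheckBounds is an unfinished stub whose branch does nothing.
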(event EventBeginPlay
  (bind _assnake_game_mode (Utilities|Casting|CastToSnakeGameMode (Game|GetGameMode)))
  (Variables|Default|SetStep (Variables|/Game/Blueprints/SnakeGameMode.SnakeGameMode_C|GetStep _assnake_game_mode))
  (Variables|Default|SetSnakeGameMode _assnake_game_mode))

(event EventTick
  (params (DeltaSeconds :type Float%20%28single-precision%29))
  (bind _returnvalue (Utilities|Time|GetRealTimeSeconds))
  (if (>= _returnvalue (Variables|Default|GetLastMoveTime))
    (Variables|Default|SetLastMoveTime (+ _returnvalue (Variables|Default|GetMoveFrequency)))
    (CallFunction|MovetoCell (+ (Variables|Default|GetCurrentCell) (Variables|Default|GetMoveDirection)))))

(event Input|KeyboardEvents|D
  (params (Key :type Key%20Structure :default "None"))
  (:Pressed
    (Variables|Default|SetMoveDirection "(X=0.000000,Y=-1.000000)")))

(event Input|KeyboardEvents|A
  (params (Key :type Key%20Structure :default "None"))
  (:Pressed
    (Variables|Default|SetMoveDirection "(X=0.000000,Y=1.000000)")))

(event Input|KeyboardEvents|W
  (params (Key :type Key%20Structure :default "None"))
  (:Pressed
    (Variables|Default|SetMoveDirection "(X=-1.000000,Y=0.000000)")))

(event Input|KeyboardEvents|S
  (params (Key :type Key%20Structure :default "None"))
  (:Pressed
    (Variables|Default|SetMoveDirection "(X=1.000000,Y=0.000000)")))

(fn ConstructionScript)

(fn CheckBounds
  (bind _returnvalue (Transformation|GetActorLocation))
  (bind _snakegamemode (Variables|Default|GetSnakeGameMode))
  (bind _step (Variables|Default|GetStep))
  (bind (_x _y) (Math|Vector|BreakVector _returnvalue))
  (bind _gamefieldsize (Variables|/Game/Blueprints/SnakeGameMode.SnakeGameMode_C|GetGameFieldSize _snakegamemode))
  (bind _returnvalue_2 (* _gamefieldsize _step))
  (bind (_x_2 _y_2) (Math|Vector2D|BreakVector2D _returnvalue_2))
  (if (or (or (< (* _x_2 -1.0) _x) (< (* _y_2 -1.0) _y)) (or (> _x_2 _x) (> _y_2 _y)))
    _))

(fn MovetoCell
  (params (Cell :type Vector%202D%20Structure))
  (bind (_x _y) (Math|Vector2D|BreakVector2D Cell))
  (bind _snakegamemode (Variables|Default|GetSnakeGameMode))
  (bind _gamefieldsize (Variables|/Game/Blueprints/SnakeGameMode.SnakeGameMode_C|GetGameFieldSize _snakegamemode))
  (bind _returnvalue (- _gamefieldsize "(X=1.000000,Y=1.000000)"))
  (bind (_x_2 _y_2) (Math|Vector2D|BreakVector2D _returnvalue))
  (bind _output_get (Variables|Default|SetCurrentCell (Math|Vector2D|MakeVector2D (Math|Float|Clamp(Float) _x 0.0 _x_2) (Math|Float|Clamp(Float) _y 0.0 _y_2))))
  (bind _position (Default|CelltoPosition (Variables|Default|GetSnakeGameMode) _output_get))
  (Transformation|SetActorLocation _position false false))